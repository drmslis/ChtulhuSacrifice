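; BP_RangeAttacksV3 performs a basic ranged attack, launching a projectile from an instigator at a target enemy.
; BasicRangeAttack spawns a BP_ProjectileBase subclass and snaps it to the given socket.
; With a montage, a notify triggers detach and Throw; without one, both happen immediately, as in V2.
; The projectile rotates toward the hard-coded ChestTarget socket, while its throw direction uses the passed-in target socket.
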(event Custom|BasicRangeAttack
  (params (EnemyToShoot :type Character%20Object%20Reference) (AttackInstigator :type Character%20Object%20Reference) (ParentComponent :type Scene%20Component%20Object%20Reference) (SocketNameToSpawnProjectile :type Name) (SocketnameToTaget :type Name) (ProjectileClass :type Object%20Class%20Reference) (MontageToPlay :type Anim%20Montage%20Object%20Reference))
  (Utilities|IsValid EnemyToShoot
    (:Is%20Valid
      (Utilities|IsValid MontageToPlay
        (:Is%20Valid
          (Variables|Default|SetTargetedEnemy EnemyToShoot)
          (Variables|Default|SetInstigator AttackInstigator)
          (bind _asbp_projectile_base (Utilities|Casting|CastToBP_ProjectileBaseClass ProjectileClass))
          (bind _returnvalue (Game|SpawnActorfromClass _asbp_projectile_base (Math|Transform|MakeTransform (Transformation|GetActorLocation (Variables|Default|GetInstigator)) (Transformation|GetActorRotation (Variables|Default|GetInstigator)) "0.200000,0.200000,0.200000") "AlwaysSpawn" (Variables|Default|GetInstigator) (Variables|Default|GetInstigator) 0))
          (Variables|Default|SetProjectileRef _returnvalue)
          (Transformation|AttachComponentToComponent (Variables|Default|GetProjectileRef) ParentComponent SocketNameToSpawnProjectile "SnapToTarget" "SnapToTarget" "KeepWorld" false)
          (Animation|Montage|PlayMontage (Actor|GetComponentbyClass (Variables|Default|GetInstigator) "/Script/Engine.SkeletalMeshComponent") MontageToPlay
            (:OnNotifyBegin
              (Transformation|DetachFromActor (Variables|Default|GetProjectileRef) "KeepWorld" "KeepWorld" "KeepRelative")
              (Transformation|SetActorRotation (Variables|Default|GetProjectileRef) (Math|Rotator|FindLookatRotation (Transformation|GetActorLocation (Variables|Default|GetProjectileRef)) (Transformation|GetSocketLocation (Utilities|Array|Get(acopy) (Actor|GetComponentsByClass (Variables|Default|GetTargetedEnemy) "/Script/Engine.SkeletalMeshComponent")) "ChestTarget")) true)
              (bind _projectileref (Variables|Default|GetProjectileRef)
                (:then
                  (Default|Throw _projectileref (Math|Vector|Normalize (- (Transformation|GetSocketLocation (Utilities|Array|Get(acopy) (Actor|GetComponentsByClass (Variables|Default|GetTargetedEnemy) "/Script/Engine.SkeletalMeshComponent")) SocketnameToTaget) (Transformation|GetActorLocation (Variables|Default|GetProjectileRef))))))
                (:else)))))
        (:Is%20Not%20Valid
          ;[1 1 1] V2 Functionality, if no montage, just shoot
          (Variables|Default|SetTargetedEnemy EnemyToShoot)
          (bind _output_get (Variables|Default|SetInstigator AttackInstigator))
          (bind _asbp_projectile_base_2 (Utilities|Casting|CastToBP_ProjectileBaseClass ProjectileClass))
          (bind _returnvalue_2 (Game|SpawnActorfromClass _asbp_projectile_base_2 (Math|Transform|MakeTransform (Transformation|GetActorLocation (Variables|Default|GetInstigator)) (Transformation|GetActorRotation (Variables|Default|GetInstigator)) "0.200000,0.200000,0.200000") "AlwaysSpawn" 0 _output_get 0))
          (Variables|Default|SetProjectileRef _returnvalue_2)
          (Transformation|AttachComponentToComponent (Variables|Default|GetProjectileRef) ParentComponent SocketNameToSpawnProjectile "SnapToTarget" "SnapToTarget" "KeepRelative" false)
          (Transformation|DetachFromActor (Variables|Default|GetProjectileRef) "KeepWorld" "KeepWorld" "KeepRelative")
          (Transformation|SetActorRotation (Variables|Default|GetProjectileRef) (Math|Rotator|FindLookatRotation (Transformation|GetActorLocation (Variables|Default|GetProjectileRef)) (Transformation|GetSocketLocation (Utilities|Array|Get(acopy) (Actor|GetComponentsByClass (Variables|Default|GetTargetedEnemy) "/Script/Engine.SkeletalMeshComponent")) "ChestTarget")) true)
          (Default|Throw (Variables|Default|GetProjectileRef) (Math|Vector|Normalize (- (Transformation|GetSocketLocation (Utilities|Array|Get(acopy) (Actor|GetComponentsByClass (Variables|Default|GetTargetedEnemy) "/Script/Engine.SkeletalMeshComponent")) SocketnameToTaget) (Transformation|GetActorLocation (Variables|Default|GetProjectileRef))))))))))

(event EventBeginPlay)

(event EventTick
  (params (DeltaSeconds :type Float%20%28single-precision%29)))