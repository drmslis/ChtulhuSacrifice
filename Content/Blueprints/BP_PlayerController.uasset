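; Player controller that routes player input to the controlled ThirdPersonCharacter.
; Target lock toggle, Charge and Jump presses, plus the MoveUp axis, each cast the controlled pawn and call the matching character function.
; The controller holds no logic of its own, and input is ignored when the pawn is not a ThirdPersonCharacter.
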(event EventBeginPlay)

(event EventTick
  (params (DeltaSeconds :type Float%20%28single-precision%29)))

(event Input|ActionEvents|InputActionLockUnlockTarget
  (params (Key :type Key%20Structure :default "None"))
  (:Pressed
    (bind _asthird_person_character (Utilities|Casting|CastToThirdPersonCharacter (Pawn|GetControlledPawn)))
    (Default|LockUnlockCharacterTarget _asthird_person_character)))

(event Input|ActionEvents|InputActionCharge
  (params (Key :type Key%20Structure :default "None"))
  (:Pressed
    (bind _asthird_person_character (Utilities|Casting|CastToThirdPersonCharacter (Pawn|GetControlledPawn)))
    (Default|Charge _asthird_person_character)))

(event Input|ActionEvents|InputActionJump
  (params (Key :type Key%20Structure :default "None"))
  (:Pressed
    (bind _asthird_person_character (Utilities|Casting|CastToThirdPersonCharacter (Pawn|GetControlledPawn)))
    (Character|Jump _asthird_person_character)))

(event Input|AxisEvents|InputAxisMoveUp
  (params (AxisValue :type Float%20%28single-precision%29))
  (bind _asthird_person_character (Utilities|Casting|CastToThirdPersonCharacter (Pawn|GetControlledPawn)))
  (Default|MoveUp _asthird_person_character AxisValue))

(fn ConstructionScript)