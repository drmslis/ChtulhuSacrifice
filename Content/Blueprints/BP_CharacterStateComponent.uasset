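; Character state component that tracks health, death and combat status.
; Health starts at MaxHealth, and Tick applies regeneration out of combat, though its use of Max rather than Min restores at least full health in one frame.
; TakeDamage subtracts damage or, when it is lethal, sets IsDead without changing CurrentHealth.
; A setter event controls the combat flag, and getters expose both flags.
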(event Custom|SetIsInCombat
  (params (bIsInCombat :type Boolean))
  (Variables|Default|SetbIsInCombat bIsInCombat))

(event EventBeginPlay
  (Variables|Default|SetCurrentHealth (Variables|Default|GetMaxHealth)))

(event EventTick
  (params (DeltaSeconds :type Float%20%28single-precision%29))
  (if (and (not (Variables|Default|GetbIsInCombat)) (< (Variables|Default|GetCurrentHealth) (Variables|Default|GetMaxHealth)))
    (Variables|Default|SetCurrentHealth (Math|Float|Max(Float) (+ (Variables|Default|GetCurrentHealth) (* DeltaSeconds (Variables|Default|GetHealthRegeneration))) (Variables|Default|GetMaxHealth)))))

(fn TakeDamage
  (params (IncomingDamage :type Float%20%28single-precision%29))
  (if (>= IncomingDamage (Variables|Default|GetCurrentHealth))
    (Variables|Default|SetbIsDead true)
    (else
      (Variables|Default|SetCurrentHealth (- (Variables|Default|GetCurrentHealth) IncomingDamage)))))

(fn GetIsDead
  (return (Variables|Default|GetbIsDead)))

(fn GetIsinCombat
  (return (Variables|Default|GetbIsInCombat)))