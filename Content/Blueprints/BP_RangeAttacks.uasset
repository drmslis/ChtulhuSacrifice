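; BP_RangeAttacks provides a BasicThrow function that launches a projectile from an attacker at a target enemy.
; It spawns a scaled-down BP_ProjectileBase, snaps it to the given socket, turns the instigator toward the enemy, then detaches the projectile.
; The projectile rotates toward the enemy's hardcoded ChestTarget socket, while Throw receives a normalized direction toward the caller-supplied target socket.
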(event EventBeginPlay)

(event EventTick
  (params (DeltaSeconds :type Float%20%28single-precision%29)))

(fn BasicThrow
  (params (EnemyToShoot :type Character%20Object%20Reference) (AttackInstigator :type Character%20Object%20Reference) (ParentComponent :type Scene%20Component%20Object%20Reference) (SocketNameToSpawnProjectile :type Name) (SocketnameToTaget :type Name))
  (Utilities|IsValid EnemyToShoot
    (:Is%20Valid
      (LocalVariables|SetTargetedEnemy EnemyToShoot)
      (LocalVariables|SetInstigator AttackInstigator)
      (bind _returnvalue (Game|SpawnActorfromClass "/Game/Blueprints/BP_ProjectileBase.BP_ProjectileBase_C" (Math|Transform|MakeTransform (Transformation|GetActorLocation (LocalVariables|GetInstigator)) (Transformation|GetActorRotation (LocalVariables|GetInstigator)) "0.200000,0.200000,0.200000") "AlwaysSpawn" (LocalVariables|GetInstigator) 0))
      (LocalVariables|SetProjectileRef _returnvalue)
      (Transformation|AttachComponentToComponent (LocalVariables|GetProjectileRef) ParentComponent SocketNameToSpawnProjectile "SnapToTarget" "SnapToTarget" "KeepRelative" true)
      (Transformation|SetActorRotation (LocalVariables|GetInstigator) (Math|Rotator|FindLookatRotation (Transformation|GetActorLocation (LocalVariables|GetInstigator)) (Transformation|GetActorLocation (LocalVariables|GetTargetedEnemy))) true)
      (Transformation|DetachFromActor (LocalVariables|GetProjectileRef) "KeepWorld" "KeepWorld" "KeepRelative")
      (Transformation|SetActorRotation (LocalVariables|GetProjectileRef) (Math|Rotator|FindLookatRotation (Transformation|GetActorLocation (LocalVariables|GetProjectileRef)) (Transformation|GetSocketLocation (Utilities|Array|Get(acopy) (Actor|GetComponentsByClass (LocalVariables|GetTargetedEnemy) "/Script/Engine.SkeletalMeshComponent")) "ChestTarget")) true)
      (Default|Throw (LocalVariables|GetProjectileRef) (Math|Vector|Normalize (- (Transformation|GetSocketLocation (Utilities|Array|Get(acopy) (Actor|GetComponentsByClass (LocalVariables|GetTargetedEnemy) "/Script/Engine.SkeletalMeshComponent")) SocketnameToTaget) (Transformation|GetActorLocation (LocalVariables|GetProjectileRef))))))))