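; BP_Boat is a boat actor that spawns fishermen when the player character enters its SpawnFisher trigger.
; The overlap spawns a pair of BP_FisherMan just above the boat at random yaw, each launched forward by a velocity-change impulse.
; A named timer then holds a cooldown flag until it resets.
; Tick prints the remaining cooldown on screen as debug output.
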(event OnComponentBeginOverlap(SpawnFisher)
  (params (OverlappedComponent :type Primitive%20Component%20Object%20Reference) (OtherActor :type Actor%20Object%20Reference) (OtherComp :type Primitive%20Component%20Object%20Reference) (OtherBodyIndex :type Integer) (bFromSweep :type Boolean) (SweepResult :type Hit%20Result%20Structure%20%28by%20ref%29))
  (Utilities|Casting|CastToTestThirdPersonCharacter1 OtherActor)
  (CallFunction|SpawnFishernam))

(event Custom|SpawnFishernam
  (bind _returnvalue (Transformation|GetActorLocation))
  (bind (_x _y _z) (Math|Vector|BreakVector _returnvalue))
  (if (not (Variables|Default|GetIsOnCD))
    (for _index (range 0 1)
      (bind _returnvalue_2 (Game|SpawnActorfromClass "/Game/Blueprints/BP_FisherMan.BP_FisherMan_C" (Math|Transform|MakeTransform (Math|Vector|MakeVector _x _y (+ _z 1.2e+02)) (Math|Rotator|MakeRotator 0.0 0.0 (Math|Random|RandomFloatinRange 0.0 359.0)) "1,1,1") "AlwaysSpawn" 0 0))
      (Physics|AddImpulse (Variables|/Script/Engine.Character|GetCharacterMovement _returnvalue_2) (* (Transformation|GetActorForwardVector _returnvalue_2) 3e+01) true))
    (bind _returnvalue_3 (Utilities|Time|SetTimerbyFunctionName 0 "ResetCooldown" (Variables|Default|GetCooldownTime)))
    (Variables|Default|SetTimer _returnvalue_3)
    (Variables|Default|SetIsOnCD true)))

(event Custom|ResetCooldown
  (Variables|Default|SetIsOnCD false))

(event EventBeginPlay
  (|CallParentFunction) ; This node is disabled and will not be called.\nDrag off pins to build functionality.
)

(event Collision|EventActorBeginOverlap
  (params (OtherActor :type Actor%20Object%20Reference))
  (|CallParentFunction OtherActor) ; This node is disabled and will not be called.\nDrag off pins to build functionality.
)

(event EventTick
  (params (DeltaSeconds :type Float%20%28single-precision%29))
  (|CallParentFunction DeltaSeconds)
  (Development|PrintString (Utilities|String|ToString(Float) (Utilities|Time|GetTimerRemainingTimebyHandle (Variables|Default|GetTimer))) true true "(R=0.000000,G=0.660000,B=1.000000,A=1.000000)" 0.0))

(fn ConstructionScript
  (|CallParentFunction))