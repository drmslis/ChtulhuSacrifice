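; BP_BaseEnemyCharacter is a base enemy character that takes damage and carries health bar and lock-on target widgets.
; ReceiveDamage flags the enemy as in combat on BPCharacterStateComponent, applies the damage there, then pushes the current health to the HealthBar widget.
; ToggleEnemyWidgets shows or hides both widgets together.
; BeginPlay, Tick, overlap, mesh hit and the construction script contain no logic.
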(event OnComponentHit(Mesh)
  (params (HitComponent :type Primitive%20Component%20Object%20Reference) (OtherActor :type Actor%20Object%20Reference) (OtherComp :type Primitive%20Component%20Object%20Reference) (NormalImpulse :type Vector :default "0, 0, 0") (Hit :type Hit%20Result%20Structure%20%28by%20ref%29)))

(event Custom|ToggleEnemyWidgets
  (params (ShowWidgets :type Boolean))
  (Rendering|SetVisibility (Variables|Default|GetHealthBar) ShowWidgets false)
  (Rendering|SetVisibility (Variables|Default|GetLockedTargetWidget) ShowWidgets false))

(event Custom|ReceiveDamage
  (params (IncomingDamage :type Float%20%28single-precision%29))
  (bind _bp_characterstatecomponent (Variables|Default|GetBP_CharacterStateComponent))
  (Default|SetIsinCombat _bp_characterstatecomponent true)
  (Default|TakeDamage _bp_characterstatecomponent IncomingDamage)
  (Default|SetHealth (.AsHealth%20Bar (Utilities|Casting|CastToHealthBar (UserInterface|GetUserWidgetObject (Variables|Default|GetHealthBar)))) (Default|GetCurrentHealth (Variables|Default|GetBP_CharacterStateComponent))))

(event EventBeginPlay)

(event Collision|EventActorBeginOverlap
  (params (OtherActor :type Actor%20Object%20Reference)))

(event EventTick
  (params (DeltaSeconds :type Float%20%28single-precision%29)))

(fn ConstructionScript)